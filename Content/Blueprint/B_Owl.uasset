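; B_Owl is the player-controlled owl in a vertical jumper, bouncing off actors tagged BRANCH.
; Each tick a short downward line trace triggers jump velocity and sound, then manual gravity and unswept offsets move it.
; MoveRight input eases horizontal speed, which is zeroed near either screen edge only while the axis is negative.
; New height records are passed to B_Sky to set the camera position.
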(event EventBeginPlay
  (bind _outactors (Actor|GetAllActorsOfClass "/Game/Blueprint/B_Sky.B_Sky_C"))
  (Variables|Default|SetSky (Utilities|Array|Get(acopy) _outactors)))

(event Collision|EventActorBeginOverlap
  (params (OtherActor :type Actor%20Object%20Reference)))

(event EventTick
  (params (DeltaSeconds :type Float%20%28single-precision%29))
  (CallFunction|CheckBranch)
  (CallFunction|MoveOwl)
  (CallFunction|SetMaxHeight))

(event Input|AxisEvents|InputAxisMoveRight
  (params (AxisValue :type Float%20%28single-precision%29))
  (CallFunction|LinearGradient AxisValue)
  (CallFunction|GetScreenSize))

(fn ConstructionScript)

(fn JumpOwl
  (Variables|Default|SetDirZ (Variables|Default|GetSpeedJump))
  (Audio|Components|Audio|Play (Variables|Default|GetJumpSound) 0.0))

(fn CheckBranch
  (bind _returnvalue (Transformation|GetActorLocation))
  (bind (_outhit _returnvalue_2) (Collision|LineTraceByChannel _returnvalue (+ _returnvalue "0, 0,-40.000000") "TraceTypeQuery3" false 0 "ForOneFrame"))
  (if _returnvalue_2
    (if (Actor|ActorHasTag (.HitActor (Collision|BreakHitResult _outhit)) "BRANCH")
      (CallFunction|JumpOwl))))

(fn GetScreenSize
  (bind _returnvalue (Game|GetPlayerController 0))
  (bind (_sizex _sizey) (HUD|GetViewportSize _returnvalue))
  (Variables|Default|SetScreenWidth (Math|Conversions|ToFloat(Integer) _sizex))
  (Variables|Default|SetScreenHeight (Math|Conversions|ToFloat(Integer) _sizey)))

(fn GetScreenPos
  (bind _returnvalue (Game|GetPlayerController 0))
  (bind _returnvalue_2 (Transformation|GetActorLocation))
  (bind _screenlocation (Class|PlayerController|ProjectWorldLocationtoScreen _returnvalue _returnvalue_2 false))
  (bind (_x _y) (Math|Vector2D|BreakVector2D _screenlocation))
  (Variables|Default|SetScreenX _x)
  (Variables|Default|SetScreenY _y))

(fn SetMaxHeight
  (bind _returnvalue (Transformation|GetActorLocation))
  (bind _z (Math|Vector|BreakVector _returnvalue))
  (if (> _z (Variables|Default|GetMaxHeight))
    (Variables|Default|SetMaxHeight _z)
    (bind _asb_sky (Utilities|Casting|CastToB_Sky (Variables|Default|GetSky)))
    (Default|SetCameraPos _asb_sky (Variables|Default|GetMaxHeight))))

(fn CheckScrLimit
  (bind _axis (Variables|Default|GetAxis))
  (bind _screenx (Variables|Default|GetScreenX))
  (CallFunction|GetScreenPos)
  (if (or (and (< _axis 0.0) (< _screenx 8e+01)) (and (< _axis 0.0) (> _screenx (- (Variables|Default|GetScreenWidth) 8e+01))))
    (Variables|Default|SetDirX 0.0)))

(fn LinearGradient
  (params (AxisValue :type Float%20%28single-precision%29))
  (bind _output_get (Variables|Default|SetAxis AxisValue))
  (Variables|Default|SetDirX (Math|Interpolation|FInterpTo (Variables|Default|GetDirX) (* _output_get (Variables|Default|GetSpeedMove)) (Utilities|Time|GetWorldDeltaSeconds) 6.0))
  (CallFunction|CheckScrLimit))

(fn MoveOwl
  (bind _output_get (Variables|Default|SetDirZ (- (Variables|Default|GetDirZ) (* (Variables|Default|GetGravity) (Utilities|Time|GetWorldDeltaSeconds)))))
  (Transformation|AddActorLocalOffset (* (Math|Vector|MakeVector (Variables|Default|GetDirX) 0.0 _output_get) (Utilities|Time|GetWorldDeltaSeconds)) false false))