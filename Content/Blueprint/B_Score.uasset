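; B_Score is an actor that displays a colored score number through a text render component.
; The construction script creates a dynamic instance of M_Score, and SetScore formats the integer and applies the color.
; BeginPlay calls SetScore with a hard-coded number and red tint.
; A timeline meant to drive material alpha, float the actor upward and destroy it when finished is never started.
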(event EventBeginPlay
  (CallFunction|SetScore 12345678 "(R=0.754167,G=0.116722,B=0.152752,A=1.000000)"))

(event Collision|EventActorBeginOverlap
  (params (OtherActor :type Actor%20Object%20Reference)))

(event EventTick
  (params (DeltaSeconds :type Float%20%28single-precision%29)))

(fn ConstructionScript
  (bind _returnvalue (Rendering|Material|CreateDynamicMaterialInstance (Variables|Default|GetScore) 0 "/Game/Material/M_Score.M_Score" "None" :!class /Script/Engine.PrimitiveComponent))
  (Variables|Default|SetFontInstance _returnvalue))

(fn SetScore
  (params (Score :type Integer) (Color :type Linear%20Color%20Structure))
  (Rendering|Components|TextRender|SetText (Variables|Default|GetScore) (Utilities|Text|FormatText "{Currency}" (Utilities|Text|ToText(Integer) Score)))
  (Rendering|Components|TextRender|SetTextRenderColor (Variables|Default|GetScore) (Math|Conversions|ToColor(LinearColor) Color)))