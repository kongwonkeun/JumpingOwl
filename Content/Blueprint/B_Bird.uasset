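; B_Bird is a flying bird actor that moves along +X and drops when it overlaps B_Owl.
; Construction randomizes speed and animation rate and creates a dynamic material, whose Index parameter Tick increments to animate the bird.
; An owl hit stops animation, rotates the bird, plays a sound and sends it downward.
; Tick also projects its location to screen space, destroying it when screen X exceeds the padded viewport width or height.
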(event EventBeginPlay
  (CallFunction|GetScreenSize))

(event Collision|EventActorBeginOverlap
  (params (OtherActor :type Actor%20Object%20Reference))
  (if (Utilities|Enum|Equal(Enum) (Utilities|GetDisplayName OtherActor) "B_Owl")
    (Utilities|FlowControl|DoOnce false
      (:Completed
        (CallFunction|DropBird)))))

(event EventTick
  (params (DeltaSeconds :type Float%20%28single-precision%29))
  (CallFunction|MoveBird)
  (CallFunction|GetScreenPos)
  (CallFunction|CheckDestroy)
  (CallFunction|AnimBird))

(fn ConstructionScript
  (bind _returnvalue (Rendering|Material|CreateDynamicMaterialInstance (Variables|Default|GetBird) 0 "/Game/Material/M_Bird.M_Bird" "None" :!class /Script/Engine.PrimitiveComponent))
  (Variables|Default|SetBirdInstance _returnvalue)
  (CallFunction|InitBird))

(fn InitBird
  (bind _returnvalue (Math|Random|RandomFloatinRange 12.0 18.0))
  (Variables|Default|SetAnimPerSec _returnvalue)
  (Variables|Default|SetAnimDelay (/ 1.0 _returnvalue))
  (Variables|Default|SetSpeed (Math|Random|RandomFloatinRange 3e+02 6e+02))
  (Variables|Default|SetDir "1.000000, 0, 0"))

(fn GetScreenSize
  (bind _returnvalue (Game|GetPlayerController 0))
  (bind (_sizex _sizey) (HUD|GetViewportSize _returnvalue))
  (Variables|Default|SetScreenWidth (Math|Conversions|ToFloat(Integer) (+ _sizex 50)))
  (Variables|Default|SetScreenHeight (Math|Conversions|ToFloat(Integer) (+ _sizey 50))))

(fn GetScreenPos
  (bind _returnvalue (Game|GetPlayerController 0))
  (bind _returnvalue_2 (Transformation|GetActorLocation))
  (bind _screenlocation (Class|PlayerController|ProjectWorldLocationtoScreen _returnvalue _returnvalue_2 false))
  (bind (_x _y) (Math|Vector2D|BreakVector2D _screenlocation))
  (Variables|Default|SetPosX _x)
  (Variables|Default|SetPoxY _y))

(fn CheckDestroy
  (if (or (> (Variables|Default|GetPosX) (Variables|Default|GetScreenWidth)) (> (Variables|Default|GetPosX) (Variables|Default|GetScreenHeight)))
    (Actor|DestroyActor)))

(fn SetAnimIndex
  (bind _output_get (Variables|Default|SetAnimIndex (+ (Variables|Default|GetAnimIndex) 1.0)))
  (Rendering|Material|SetScalarParameterValue (Variables|Default|GetBirdInstance) "Index" _output_get :!class /Script/Engine.MaterialInstanceDynamic))

(fn AnimBird
  (if (not (Variables|Default|GetIsDead))
    (bind _output_get (Variables|Default|SetAnimDelay (- (Variables|Default|GetAnimDelay) (Utilities|Time|GetWorldDeltaSeconds))))
    (if (< _output_get 0.0)
      (Variables|Default|SetAnimDelay (/ 1.0 (Variables|Default|GetAnimPerSec)))
      (CallFunction|SetAnimIndex))))

(fn MoveBird
  (Transformation|AddActorWorldOffset (* (Variables|Default|GetDir) (* (Variables|Default|GetSpeed) (Utilities|Time|GetWorldDeltaSeconds)))))

(fn DropBird
  (Variables|Default|SetIsDead true)
  (Transformation|SetActorRotation "180.000000, 0, 0")
  (Variables|Default|SetDir "0, 0,-1.000000")
  (Audio|PlaySoundatLocation "/Game/Audio/bird.bird" (Transformation|GetActorLocation) "0, 0, 0" 1.0 1.0 0.0 0 0 0))