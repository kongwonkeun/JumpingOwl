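; B_Gift is a gift actor that shows one of three random images and destroys itself when anything overlaps it.
; Its construction script creates a dynamic instance of M_Gift and randomly sets the GiftImage texture parameter.
; Every tick it projects its location to screen space and destroys itself once it passes slightly below the bottom of the viewport.
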(event EventBeginPlay)

(event Collision|EventActorBeginOverlap
  (params (OtherActor :type Actor%20Object%20Reference))
  (Actor|DestroyActor))

(event EventTick
  (params (DeltaSeconds :type Float%20%28single-precision%29))
  (CallFunction|CheckPosition))

(fn ConstructionScript
  (bind _returnvalue (Rendering|Material|CreateDynamicMaterialInstance (Variables|Default|GetGift) 0 "/Game/Material/M_Gift.M_Gift" "None" :!class /Script/Engine.PrimitiveComponent))
  (Variables|Default|SetGiftInstance _returnvalue)
  (CallFunction|SetGiftImage))

(fn SetGiftImage
  (bind _giftinstance (Variables|Default|GetGiftInstance))
  (bind _output_get (Variables|Default|SetGiftNum (Math|Random|RandomIntegerinRange 1 3)))
  (switch int _output_get
    (:1
      (Rendering|Material|SetTextureParameterValue _giftinstance "GiftImage" "/Game/Texture/gift1.gift1"))
    (:2
      (Rendering|Material|SetTextureParameterValue _giftinstance "GiftImage" "/Game/Texture/gift2.gift2"))
    (:3
      (Rendering|Material|SetTextureParameterValue _giftinstance "GiftImage" "/Game/Texture/gift3.gift3"))))

(fn CheckPosition
  (bind _returnvalue (Game|GetPlayerController 0))
  (if (> (.Y (Math|Vector2D|BreakVector2D (.ScreenLocation (Class|PlayerController|ProjectWorldLocationtoScreen _returnvalue (Transformation|GetActorLocation) false)))) (Math|Conversions|ToFloat(Integer) (+ (.SizeY (HUD|GetViewportSize _returnvalue)) 50)))
    (Actor|DestroyActor)))